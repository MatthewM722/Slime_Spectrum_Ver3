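; Trampoline actor that launches the slime player on overlap with a bounce force along Y and Z.
; Overlap sets the player's Springboard flag and opens a gate, letting Tick apply acceleration-based force every frame until the gate closes.
; Chained delays clear the flag on player pawn 0, disable the trampoline's collision, then restore it and close the gate.
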(event Collision|EventActorBeginOverlap
  (params (OtherActor :type Actor%20Object%20Reference))
  ;[1 1 1] once player interacts, activate spring board
  (bind _asslime_player (Utilities|Casting|CastToSlime_Player OtherActor))
  (Variables|/Game/Player/Slime_Player.Slime_Player_C|SetSpringboard _asslime_player true)
  ;[1 1 1] set velocity and switch player movement
  (Utilities|FlowControl|Gate true) ; enters at Open
)

(event EventTick
  (params (DeltaSeconds :type Float%20%28single-precision%29))
  ;[1 1 1] set velocity and switch player movement
  (Utilities|FlowControl|Gate true :!label _label
    (:Exit
      (Utilities|IsValid (Variables|/Game/Player/Slime_Player.Slime_Player_C|GetSlime_Player (stale Collision|EventActorBeginOverlap _asslime_player))
        (:Is%20Valid
          (Physics|AddForce (Variables|/Game/Player/Slime_Player.Slime_Player_C|GetSlime_Player (stale Collision|EventActorBeginOverlap _asslime_player)) (Math|Vector|MakeVector 0.0 (Variables|Default|GetBounce%20Y) (Variables|Default|GetBounce%20Z)) "None" true)
          (Utilities|FlowControl|Delay 0.5)
          (bind _asslime_player (Utilities|Casting|CastToSlime_Player (Game|Player|GetPlayerPawn 0)))
          (Variables|/Game/Player/Slime_Player.Slime_Player_C|Setspringboard _asslime_player false)
          (Collision|SetCollisionEnabled (Variables|Default|Getcollision) "NoCollision")
          (Utilities|FlowControl|Delay 2.0)
          (Collision|SetCollisionEnabled (Variables|Default|Getcollision) "QueryAndPhysics")
          (goto _label Close))))))

(fn ConstructionScript)