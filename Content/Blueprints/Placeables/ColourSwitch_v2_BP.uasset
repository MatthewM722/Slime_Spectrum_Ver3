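; Colour switch pickup that recolours the slime player to its own colour on overlap, doing nothing if the colours already match.
; On a switch, it passes the colour to every ConveyerBelt_BP; the same loop hides the sphere mesh and restores it after a two-second delay.
; The construction script calls UpdateColour, which maps the colour enum to a sphere material for live editor preview.
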(event Collision|EventActorBeginOverlap
  (params (OtherActor :type Actor%20Object%20Reference))
  (bind _sphere (Variables|Default|GetSphere))
  ;[1 1 1] Changes colour of the slime to the same colour as the pickup and dissapears for 2 seconds. If the colour is the same, does nothing.
  (bind _asslime_player (Utilities|Casting|CastToSlime_Player OtherActor))
  (if (not (Utilities|Enum|Equal(Enum) (Variables|Default|GetSwitcher_CurrentColour) (Variables|/Game/Player/Slime_Player.Slime_Player_C|GetSlime_CurrentColour _asslime_player)))
    (Default|UpdateColour _asslime_player (Variables|Default|GetSwitcher_CurrentColour))
    ;[0 1 0.658] Conveyer Belt
    (bind _outactors (Actor|GetAllActorsOfClass "/Game/Blueprints/Placeables/ConveyerBelt_BP.ConveyerBelt_BP_C"))
    (for _array_element _outactors
      (Class|BPIColourBelt|CallColourSwitch(Message) _array_element (Variables|Default|GetSwitcher_CurrentColour))
      (Rendering|SetVisibility _sphere false false)
      (Utilities|FlowControl|Delay 2.0)
      (Rendering|SetVisibility _sphere true false))))

(fn ConstructionScript
  ;[1 1 1] Updates Colour Live
  (CallFunction|UpdateColour (Variables|Default|GetSwitcher_CurrentColour)))

(fn UpdateColour
  (params (New%20Colour :type Colour_List%20Enum :default "NewEnumerator3"))
  (bind _sphere (Variables|Default|GetSphere))
  ;[1 1 1] Changes Colour of Pickup
  (bind _output_get (Variables|Default|SetSwitcher_CurrentColour New%20Colour))
  (switch Utilities|FlowControl|Switch|SwitchonColour_List _output_get
    (:NewEnumerator3
      (Rendering|Material|SetMaterial _sphere 0 "/Game/BlockOut/Materials_Textures/GreenColour_M.GreenColour_M"))
    (:NewEnumerator0
      (Rendering|Material|SetMaterial _sphere 0 "/Game/BlockOut/Materials_Textures/RedColour_M.RedColour_M"))
    (:NewEnumerator1
      (Rendering|Material|SetMaterial _sphere 0 "/Game/BlockOut/Materials_Textures/BlueColour_M.BlueColour_M"))
    (:NewEnumerator2
      (Rendering|Material|SetMaterial _sphere 0 "/Game/BlockOut/Materials_Textures/YellowColour_M.YellowColour_M"))
    (:NewEnumerator4
      (Rendering|Material|SetMaterial _sphere 0 "/Game/BlockOut/Materials_Textures/PinkColour_M.PinkColour_M"))
    (:NewEnumerator5
      (Rendering|Material|SetMaterial _sphere 0 "/Game/BlockOut/Materials_Textures/PurpleColour_M.PurpleColour_M"))
    (:NewEnumerator6
      (Rendering|Material|SetMaterial _sphere 0 "/Game/BlockOut/Materials_Textures/OrangeColour_M.OrangeColour_M"))))