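; Slime press hazard, a placeable trap with two halves that move in mirror image and kill the player slime.
; A looping timeline drives both halves along X in opposite directions, pausing for a Delay between cycles.
; The collider is active only while the timeline value is within a set range, and an overlap with Slime_Player calls its Death and prints a debug string.
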(event OnComponentBeginOverlap(Collider)
  (params (OverlappedComponent :type Primitive%20Component%20Object%20Reference) (OtherActor :type Actor%20Object%20Reference) (OtherComp :type Primitive%20Component%20Object%20Reference) (OtherBodyIndex :type Integer) (bFromSweep :type Boolean) (SweepResult :type Hit%20Result%20Structure%20%28by%20ref%29))
  (bind _asslime_player (Utilities|Casting|CastToSlime_Player OtherActor))
  (Default|Death _asslime_player)
  (Development|PrintString "Hello"))

(event EventBeginPlay
  (bind _transform (Timeline|Animation Play)
    (:Update
      (Transformation|SetRelativeTransform (Variables|Default|GetSlimePress_Left) (Math|Transform|MakeTransform (Math|Vector|MakeVector _transform 0.0 0.0) "0, 0, 0" "10.000000,10.000000,10.000000") false false)
      (Transformation|SetRelativeTransform (Variables|Default|GetSlimePress_Right) (Math|Transform|MakeTransform (Math|Vector|MakeVector (* _transform -1.0) 0.0 0.0) "0, 0, 0" "10.000000,10.000000,10.000000") false false)
      (if (Math|Float|InRange(Float) _transform -5.0 11.0)
        (Collision|SetCollisionEnabled (Variables|Default|GetCollider) "QueryAndPhysics")
        (else
          (Collision|SetCollisionEnabled (Variables|Default|GetCollider) "NoCollision"))))
    (:Finished
      (Utilities|FlowControl|Delay (Variables|Default|GetDelay))
      (Timeline|Animation PlayFromStart))))

(fn ConstructionScript)