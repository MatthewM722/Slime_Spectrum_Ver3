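; Placeable conveyor belt that carries the slime player along its surface.
; Each Tick it offsets every Slime_Player overlapping its Box along the static mesh's forward vector, scaled by Speed and delta time, without sweeping.
; The construction script creates a dynamic Conveyer_M material on the mesh, setting colour, arrow scale and track scroll speed.
; The visual track speed is a separate variable from the push speed.
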(event EventTick
  (params (DeltaSeconds :type Float%20%28single-precision%29))
  (for _array_element (Collision|GetOverlappingActors (Variables|Default|GetBox) "/Game/Player/Slime_Player.Slime_Player_C" :!class /Script/Engine.PrimitiveComponent)
    (Transformation|AddActorWorldOffset _array_element (* (Math|Vector|GetForwardVector (Transformation|GetWorldRotation (Variables|Default|GetStaticMesh))) (* DeltaSeconds (Variables|Default|GetSpeed))))))

(event EventBeginPlay)

(fn ConstructionScript
  (bind _staticmesh (Variables|Default|GetStaticMesh))
  (bind _returnvalue (Rendering|Material|CreateDynamicMaterialInstance _staticmesh 0 "/Game/Materials/Conveyer_M.Conveyer_M" "None" :!class /Script/Engine.PrimitiveComponent))
  (Rendering|Material|SetVectorParameterValue _returnvalue "Colour" (Variables|Default|GetColour) :!class /Script/Engine.MaterialInstanceDynamic)
  (Rendering|Material|SetMaterial _staticmesh 0 _returnvalue)
  (Rendering|Material|SetScalarParameterValue _returnvalue "x scale" (Variables|Default|GetArrow%20scale) :!class /Script/Engine.MaterialInstanceDynamic)
  (Rendering|Material|SetScalarParameterValue _returnvalue "x speed" (Variables|Default|GetTrack%20speed) :!class /Script/Engine.MaterialInstanceDynamic))