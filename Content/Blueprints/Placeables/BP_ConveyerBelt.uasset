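; Placeable conveyor belt that pushes the slime player along or against its arrow direction depending on the slime's colour.
; Overlap opens a Tick-driven gate that offsets the player by ArrowLeft's forward vector times Speed, reversed for ColourLeftInverted and unchanged for ColourRightDefault.
; The construction script calls UpdateColour to tint both arrows with inverted and default dynamic materials.
; CallColourSwitch is empty, and an older colour-to-speed switch is left disconnected.
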(event OnComponentBeginOverlap(Collision)
  (params (OverlappedComponent :type Primitive%20Component%20Object%20Reference) (OtherActor :type Actor%20Object%20Reference) (OtherComp :type Primitive%20Component%20Object%20Reference) (OtherBodyIndex :type Integer) (bFromSweep :type Boolean) (SweepResult :type Hit%20Result%20Structure%20%28by%20ref%29))
  (bind _asslime_player (Utilities|Casting|CastToSlime_Player OtherActor))
  (Variables|Default|SetReference_SlimePlayer _asslime_player)
  (CallFunction|OpenGate))

(event OnComponentEndOverlap(Collision)
  (params (OverlappedComponent :type Primitive%20Component%20Object%20Reference) (OtherActor :type Actor%20Object%20Reference) (OtherComp :type Primitive%20Component%20Object%20Reference) (OtherBodyIndex :type Integer))
  (Utilities|Casting|CastToSlime_Player OtherActor)
  (CallFunction|CloseGate))

(event Custom|CloseGate
  ;[1 0.1521 0.158] Conveyer Belt Movement
  (Utilities|FlowControl|Gate true) ; enters at Close
)

(event Custom|OpenGate
  ;[1 0.1521 0.158] Conveyer Belt Movement
  (Utilities|FlowControl|Gate true) ; enters at Open
)

(event EventCallColourSwitch
  (params (Switch%20to%20this%20colour :type Colour_List%20Enum :default "NewEnumerator3"))
  ;[0.1604 0.1684 1] Colour pick up changes
)

(event EventTick
  (params (DeltaSeconds :type Float%20%28single-precision%29))
  (bind _speed (Variables|Default|GetSpeed))
  (bind _arrowleft (Variables|Default|GetArrowLeft))
  (bind _returnvalue (Transformation|GetWorldRotation _arrowleft))
  (bind _returnvalue_2 (* DeltaSeconds _speed))
  (bind _returnvalue_3 (Math|Vector|GetForwardVector _returnvalue))
  (bind _returnvalue_4 (* _returnvalue_3 _returnvalue_2))
  ;[1 0.1521 0.158] Conveyer Belt Movement
  (Utilities|FlowControl|Gate true
    (:Exit
      (if (Utilities|Enum|Equal(Enum) (Variables|/Game/Player/Slime_Player.Slime_Player_C|GetSlime_CurrentColour (Variables|Default|GetReference_SlimePlayer)) (Variables|Default|GetColourLeft%20/%20Inverted))
        (Transformation|AddActorWorldOffset (Variables|Default|GetReference_SlimePlayer) (* _returnvalue_4 "-1.000000,-1.000000,-1.000000"))
        (elif (Utilities|Enum|Equal(Enum) (Variables|/Game/Player/Slime_Player.Slime_Player_C|GetSlime_CurrentColour (Variables|Default|GetReference_SlimePlayer)) (Variables|Default|GetColourRight%20/%20Default))
          (Transformation|AddActorWorldOffset (Variables|Default|GetReference_SlimePlayer) _returnvalue_4))))))

(fn ConstructionScript
  (bind _returnvalue (Rendering|Material|CreateDynamicMaterialInstance (Variables|Default|GetArrowLeft) 0 "/Game/Materials/Conveyer_Belt/Conveyer_M.Conveyer_M" "None" :!class /Script/Engine.PrimitiveComponent))
  (Rendering|Material|SetVectorParameterValue _returnvalue "Colour" (Variables|Default|GetColour) :!class /Script/Engine.MaterialInstanceDynamic)
  (Rendering|Material|SetMaterial (Variables|Default|GetArrowLeft) 0 _returnvalue)
  (Rendering|Material|SetScalarParameterValue _returnvalue "x scale" (Variables|Default|GetArrow%20scale) :!class /Script/Engine.MaterialInstanceDynamic)
  (Rendering|Material|SetScalarParameterValue _returnvalue "x speed" (Variables|Default|GetTrack%20speed) :!class /Script/Engine.MaterialInstanceDynamic)
  (CallFunction|UpdateColour (Variables|Default|GetColourLeft%20/%20Inverted) (Variables|Default|GetColourRight%20/%20Default)))

(fn UpdateColour
  (params (Colour1 :type Colour_List%20Enum :default "NewEnumerator3") (Colour2 :type Colour_List%20Enum :default "NewEnumerator3"))
  (bind _arrowleft (Variables|Default|GetArrowLeft))
  (bind _arrowright (Variables|Default|GetArrowRight))
  (bind _output_get (Variables|Default|SetColourLeft%20/%20Inverted Colour1))
  (switch Utilities|FlowControl|Switch|SwitchonColour_List _output_get
    (:NewEnumerator3
      (bind _returnvalue (Rendering|Material|CreateDynamicMaterialInstance _arrowleft 0 "/Game/Materials/Conveyer_Belt/Conveyer_Inverted_M.Conveyer_Inverted_M" "None" :!class /Script/Engine.PrimitiveComponent))
      (bind _output_get_2 (Variables|Default|SetColour "(R=0.000000,G=0.352941,B=0.007843,A=1.000000)"))
      (Rendering|Material|SetVectorParameterValue _returnvalue "Colour" _output_get_2 :!class /Script/Engine.MaterialInstanceDynamic))
    (:NewEnumerator0
      (bind _returnvalue_2 (Rendering|Material|CreateDynamicMaterialInstance _arrowleft 0 "/Game/Materials/Conveyer_Belt/Conveyer_Inverted_M.Conveyer_Inverted_M" "None" :!class /Script/Engine.PrimitiveComponent))
      (bind _output_get_3 (Variables|Default|SetColour "(R=0.672917,G=0.000000,B=0.054809,A=1.000000)"))
      (Rendering|Material|SetVectorParameterValue _returnvalue_2 "Colour" _output_get_3 :!class /Script/Engine.MaterialInstanceDynamic))
    (:NewEnumerator1
      (bind _returnvalue_3 (Rendering|Material|CreateDynamicMaterialInstance _arrowleft 0 "/Game/Materials/Conveyer_Belt/Conveyer_Inverted_M.Conveyer_Inverted_M" "None" :!class /Script/Engine.PrimitiveComponent))
      (bind _output_get_4 (Variables|Default|SetColour "(R=0.034969,G=0.106459,B=1.000000,A=1.000000)"))
      (Rendering|Material|SetVectorParameterValue _returnvalue_3 "Colour" _output_get_4 :!class /Script/Engine.MaterialInstanceDynamic))
    (:NewEnumerator2
      (bind _returnvalue_4 (Rendering|Material|CreateDynamicMaterialInstance _arrowleft 0 "/Game/Materials/Conveyer_Belt/Conveyer_Inverted_M.Conveyer_Inverted_M" "None" :!class /Script/Engine.PrimitiveComponent))
      (bind _output_get_5 (Variables|Default|SetColour "(R=1.000000,G=0.966980,B=0.000000,A=1.000000)"))
      (Rendering|Material|SetVectorParameterValue _returnvalue_4 "Colour" _output_get_5 :!class /Script/Engine.MaterialInstanceDynamic))
    (:NewEnumerator4
      (bind _returnvalue_5 (Rendering|Material|CreateDynamicMaterialInstance _arrowleft 0 "/Game/Materials/Conveyer_Belt/Conveyer_Inverted_M.Conveyer_Inverted_M" "None" :!class /Script/Engine.PrimitiveComponent))
      (bind _output_get_6 (Variables|Default|SetColour "(R=1.000000,G=0.016720,B=0.850006,A=1.000000)"))
      (Rendering|Material|SetVectorParameterValue _returnvalue_5 "Colour" _output_get_6 :!class /Script/Engine.MaterialInstanceDynamic))
    (:NewEnumerator5
      (bind _returnvalue_6 (Rendering|Material|CreateDynamicMaterialInstance _arrowleft 0 "/Game/Materials/Conveyer_Belt/Conveyer_Inverted_M.Conveyer_Inverted_M" "None" :!class /Script/Engine.PrimitiveComponent))
      (bind _output_get_7 (Variables|Default|SetColour "(R=0.190376,G=0.000000,B=1.000000,A=1.000000)"))
      (Rendering|Material|SetVectorParameterValue _returnvalue_6 "Colour" _output_get_7 :!class /Script/Engine.MaterialInstanceDynamic))
    (:NewEnumerator6
      (bind _returnvalue_7 (Rendering|Material|CreateDynamicMaterialInstance _arrowleft 0 "/Game/Materials/Conveyer_Belt/Conveyer_Inverted_M.Conveyer_Inverted_M" "None" :!class /Script/Engine.PrimitiveComponent))
      (bind _output_get_8 (Variables|Default|SetColour "(R=1.000000,G=0.198644,B=0.000000,A=1.000000)"))
      (Rendering|Material|SetVectorParameterValue _returnvalue_7 "Colour" _output_get_8 :!class /Script/Engine.MaterialInstanceDynamic)))
  (bind _output_get_9 (Variables|Default|SetColourRight%20/%20Default Colour2))
  (switch Utilities|FlowControl|Switch|SwitchonColour_List _output_get_9
    (:NewEnumerator3
      (bind _returnvalue_8 (Rendering|Material|CreateDynamicMaterialInstance _arrowright 0 "/Game/Materials/Conveyer_Belt/Conveyer_M.Conveyer_M" "None" :!class /Script/Engine.PrimitiveComponent))
      (bind _output_get_10 (Variables|Default|SetColour "(R=0.000000,G=0.352941,B=0.007843,A=1.000000)"))
      (Rendering|Material|SetVectorParameterValue _returnvalue_8 "Colour" _output_get_10 :!class /Script/Engine.MaterialInstanceDynamic))
    (:NewEnumerator0
      (bind _returnvalue_9 (Rendering|Material|CreateDynamicMaterialInstance _arrowright 0 "/Game/Materials/Conveyer_Belt/Conveyer_M.Conveyer_M" "None" :!class /Script/Engine.PrimitiveComponent))
      (bind _output_get_11 (Variables|Default|SetColour "(R=0.672917,G=0.000000,B=0.054809,A=1.000000)"))
      (Rendering|Material|SetVectorParameterValue _returnvalue_9 "Colour" _output_get_11 :!class /Script/Engine.MaterialInstanceDynamic))
    (:NewEnumerator1
      (bind _returnvalue_10 (Rendering|Material|CreateDynamicMaterialInstance _arrowright 0 "/Game/Materials/Conveyer_Belt/Conveyer_M.Conveyer_M" "None" :!class /Script/Engine.PrimitiveComponent))
      (bind _output_get_12 (Variables|Default|SetColour "(R=0.034969,G=0.106459,B=1.000000,A=1.000000)"))
      (Rendering|Material|SetVectorParameterValue _returnvalue_10 "Colour" _output_get_12 :!class /Script/Engine.MaterialInstanceDynamic))
    (:NewEnumerator2
      (bind _returnvalue_11 (Rendering|Material|CreateDynamicMaterialInstance _arrowright 0 "/Game/Materials/Conveyer_Belt/Conveyer_M.Conveyer_M" "None" :!class /Script/Engine.PrimitiveComponent))
      (bind _output_get_13 (Variables|Default|SetColour "(R=1.000000,G=0.966980,B=0.000000,A=1.000000)"))
      (Rendering|Material|SetVectorParameterValue _returnvalue_11 "Colour" _output_get_13 :!class /Script/Engine.MaterialInstanceDynamic))
    (:NewEnumerator4
      (bind _returnvalue_12 (Rendering|Material|CreateDynamicMaterialInstance _arrowright 0 "/Game/Materials/Conveyer_Belt/Conveyer_M.Conveyer_M" "None" :!class /Script/Engine.PrimitiveComponent))
      (bind _output_get_14 (Variables|Default|SetColour "(R=1.000000,G=0.016720,B=0.850006,A=1.000000)"))
      (Rendering|Material|SetVectorParameterValue _returnvalue_12 "Colour" _output_get_14 :!class /Script/Engine.MaterialInstanceDynamic))
    (:NewEnumerator5
      (bind _returnvalue_13 (Rendering|Material|CreateDynamicMaterialInstance _arrowright 0 "/Game/Materials/Conveyer_Belt/Conveyer_M.Conveyer_M" "None" :!class /Script/Engine.PrimitiveComponent))
      (bind _output_get_15 (Variables|Default|SetColour "(R=0.190376,G=0.000000,B=1.000000,A=1.000000)"))
      (Rendering|Material|SetVectorParameterValue _returnvalue_13 "Colour" _output_get_15 :!class /Script/Engine.MaterialInstanceDynamic))
    (:NewEnumerator6
      (bind _returnvalue_14 (Rendering|Material|CreateDynamicMaterialInstance _arrowright 0 "/Game/Materials/Conveyer_Belt/Conveyer_M.Conveyer_M" "None" :!class /Script/Engine.PrimitiveComponent))
      (bind _output_get_16 (Variables|Default|SetColour "(R=1.000000,G=0.198644,B=0.000000,A=1.000000)"))
      (Rendering|Material|SetVectorParameterValue _returnvalue_14 "Colour" _output_get_16 :!class /Script/Engine.MaterialInstanceDynamic))))