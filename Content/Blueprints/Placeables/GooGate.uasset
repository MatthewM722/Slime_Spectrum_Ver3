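; GooGate is a placeable colour gate that lets a Slime_Player through only when the slime's colour matches the gate's.
; On actor overlap it compares the two colours and disables the Collision component on a match, or enables query and physics collision otherwise.
; The construction script calls UpdateColour, which sets the gate mesh material from GateCurrentColour.
; An older per-colour boolean check remains in the event graph but never runs.
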(event Collision|EventActorBeginOverlap
  (params (OtherActor :type Actor%20Object%20Reference))
  ;[1 1 1] Matthews Colour Gate
  (bind _asslime_player (Utilities|Casting|CastToSlime_Player OtherActor))
  (if (Utilities|Enum|Equal(Enum) (Variables|Default|GetGate_CurrentColour) (Variables|/Game/Player/Slime_Player.Slime_Player_C|GetSlime_CurrentColour _asslime_player))
    (Collision|SetCollisionEnabled (Variables|Default|Getcollision) "NoCollision")
    (Development|PrintString "Hello")
    (else
      (Collision|SetCollisionEnabled (Variables|Default|Getcollision) "QueryAndPhysics"))))

(fn ConstructionScript
  (CallFunction|UpdateColour (Variables|Default|GetGate_CurrentColour)))

(fn UpdateColour
  (params (New%20Colour :type Colour_List%20Enum :default "NewEnumerator3"))
  ;[1 1 1] Changes Colour of Gate
  (bind _output_get (Variables|Default|SetGate_CurrentColour New%20Colour))
  (switch Utilities|FlowControl|Switch|SwitchonColour_List _output_get
    (:NewEnumerator3
      (Rendering|Material|SetMaterial (Variables|Default|GetSlime_Gate) 0 "/Game/Assets/Slime_Gate/Materials/Slime_Material_Green.Slime_Material_Green"))
    (:NewEnumerator0
      (Rendering|Material|SetMaterial (Variables|Default|GetSlime_Gate) 0 "/Game/Assets/Slime_Gate/Materials/Slime_Material_Red.Slime_Material_Red"))
    (:NewEnumerator1
      (Rendering|Material|SetMaterial (Variables|Default|GetSlime_Gate) 0 "/Game/Assets/Slime_Gate/Materials/Slime_Material_Blue.Slime_Material_Blue"))
    (:NewEnumerator2
      (Rendering|Material|SetMaterial (Variables|Default|GetSlime_Gate) 0 "/Game/Assets/Slime_Gate/Materials/Slime_Material_Yellow.Slime_Material_Yellow"))
    (:NewEnumerator4
      (Rendering|Material|SetMaterial (Variables|Default|GetSlime_Gate) 0 "/Game/Assets/Slime_Gate/Materials/Slime_Material_Pink.Slime_Material_Pink"))
    (:NewEnumerator5
      (Rendering|Material|SetMaterial (Variables|Default|GetSlime_Gate) 0 "/Game/Textures/Materials/Purple.Purple"))
    (:NewEnumerator6
      (Rendering|Material|SetMaterial (Variables|Default|GetSlime_Gate) 0 "/Game/Textures/Materials/Orange.Orange"))))