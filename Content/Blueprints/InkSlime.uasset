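; InkSlime is an actor that rises along a spline path, apparently as a rising ink hazard.
; On BeginPlay it finds a SplinePathBP in the level and plays the Moveobject timeline at a rate derived from Timetocomplete.
; Each update sets world location and local-space rotation from the distance along the spline, with a fixed enlarged scale.
; An older MoveComponentTo up-and-return chain is left unconnected, and inkrising is empty.
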(event Custom|ink%20rising)

(event Custom|riseup
  (bind _splineref (Variables|Default|Getsplineref))
  (bind _spline (Variables|/Game/Blueprints/splinePathBP.splinePathBP_C|GetSpline _splineref))
  (Components|Timeline|SetPlayRate (Variables|Default|Getmoveobject) (/ 1.0 (Variables|Default|Gettimetocomplete)))
  (bind _move (Timeline|moveobject Play)
    (:Update
      (Transformation|SetActorTransform (Math|Transform|MakeTransform (Spline|GetLocationatDistanceAlongSpline _spline (Math|Float|Lerp 0.0 (Spline|GetSplineLength (Variables|/Game/Blueprints/splinePathBP.splinePathBP_C|GetSpline (Variables|Default|Getsplineref))) _move) "World") (Spline|GetRotationatDistanceAlongSpline _spline (Math|Float|Lerp 0.0 (Spline|GetSplineLength (Variables|/Game/Blueprints/splinePathBP.splinePathBP_C|GetSpline (Variables|Default|Getsplineref))) _move) "Local") "10.750000,10.750000,10.750000")))))

(event EventBeginPlay
  (bind _returnvalue (Actor|GetActorOfClass "/Game/Blueprints/splinePathBP.splinePathBP_C"))
  (Variables|Default|Setsplineref _returnvalue)
  (CallFunction|Riseup))

(event Collision|EventActorBeginOverlap
  (params (OtherActor :type Actor%20Object%20Reference)))

(event EventTick
  (params (DeltaSeconds :type Float%20%28single-precision%29)))

(fn ConstructionScript)