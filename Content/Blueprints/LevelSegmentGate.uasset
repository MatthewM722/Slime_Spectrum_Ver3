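; Trigger gate between level segments that pans the slime player's camera when the player passes through it.
; On overlap, an IsVertical flag selects the Z or Y axis, and the sign of the player's velocity on it sets the pan direction.
; It also calls the matching Up, Down, Left or Right event on the first Enemy_pawn found in the world, if one exists.
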(event OnComponentBeginOverlap(Collider)
  (params (OverlappedComponent :type Primitive%20Component%20Object%20Reference) (OtherActor :type Actor%20Object%20Reference) (OtherComp :type Primitive%20Component%20Object%20Reference) (OtherBodyIndex :type Integer) (bFromSweep :type Boolean) (SweepResult :type Hit%20Result%20Structure%20%28by%20ref%29))
  (bind _asslime_player (Utilities|Casting|CastToSlime_Player OtherActor))
  (Variables|Default|SetRef_SlimePlayer _asslime_player)
  (if (Variables|Default|GetIsVertical)
    (if (> (.z (Transformation|GetVelocity (Variables|Default|GetRef_SlimePlayer))) 0.0)
      (Default|PanCamera (Variables|Default|GetRef_SlimePlayer) "NewEnumerator0")
      (bind _returnvalue (Actor|GetActorOfClass "/Game/Blueprints/Boss/Enemy_pawn.Enemy_pawn_C"))
      (Utilities|IsValid _returnvalue
        (:Is%20Valid
          (Default|Up _returnvalue)))
      (else
        (Default|PanCamera (Variables|Default|GetRef_SlimePlayer) "NewEnumerator1")
        (bind _returnvalue_2 (Actor|GetActorOfClass "/Game/Blueprints/Boss/Enemy_pawn.Enemy_pawn_C"))
        (Utilities|IsValid _returnvalue_2
          (:Is%20Valid
            (Default|Down _returnvalue_2)))))
    (elif (> (.y (Transformation|GetVelocity (Variables|Default|GetRef_SlimePlayer))) 0.0)
      (Default|PanCamera (Variables|Default|GetRef_SlimePlayer) "NewEnumerator3")
      (bind _returnvalue_3 (Actor|GetActorOfClass "/Game/Blueprints/Boss/Enemy_pawn.Enemy_pawn_C"))
      (Utilities|IsValid _returnvalue_3
        (:Is%20Valid
          (Default|Right _returnvalue_3)))
      (else
        (Default|PanCamera (Variables|Default|GetRef_SlimePlayer) "NewEnumerator2")
        (bind _returnvalue_4 (Actor|GetActorOfClass "/Game/Blueprints/Boss/Enemy_pawn.Enemy_pawn_C"))
        (Utilities|IsValid _returnvalue_4
          (:Is%20Valid
            (Default|Left _returnvalue_4)))))))

(fn ConstructionScript)