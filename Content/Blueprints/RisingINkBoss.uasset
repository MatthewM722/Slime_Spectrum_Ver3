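; RisingINkBoss is a hazard actor of rising ink that kills the player on contact.
; Shortly after BeginPlay it sets the Ink component to a thin, wide scale and triggers its rise event.
; A timeline then drives a Lerp on the ink's Z scale, growing it far taller over time.
; Any overlapping Slime_Player has its Death function called.
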(event Custom|rise
  (bind _inkscale (Timeline|inkrise Play)
    (:Update
      (Transformation|SetRelativeScale3D (Variables|Default|Getink) (Math|Vector|MakeVector 1.0 36.0 (Math|Float|Lerp 1.0 9e+01 _inkscale))))))

(event EventBeginPlay
  (Utilities|FlowControl|Delay 0.5)
  (Transformation|SetRelativeScale3D (Variables|Default|Getink) (Math|Vector|MakeVector 1.0 14.0 0.25))
  (CallFunction|Rise))

(event Collision|EventActorBeginOverlap
  (params (OtherActor :type Actor%20Object%20Reference))
  (bind _asslime_player (Utilities|Casting|CastToSlime_Player OtherActor))
  (Default|Death _asslime_player))

(event EventTick
  (params (DeltaSeconds :type Float%20%28single-precision%29)))

(fn ConstructionScript)