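; Behavior tree task for the boss that swings the enemy pawn's left saw arm in an attack.
; MoveComponentTo rolls SawArmleft a half turn from its current world roll, applied as a relative rotation, while keeping its location.
; A parallel delay triggers Return just before the move ends, reversing the swing.
; The move's Completed output prints a debug string and finishes the task successfully.
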(event EventReceiveExecuteAI
  (params (OwnerController :type AI%20Controller%20Object%20Reference) (ControlledPawn :type Pawn%20Object%20Reference))
  (bind _asenemy_pawn (Utilities|Casting|CastToEnemy_pawn ControlledPawn))
  (bind _output_get (Variables|Default|Setdefaultrotation (.roll (Transformation|GetWorldRotation (Variables|/Game/Blueprints/Boss/Enemy_pawn.Enemy_pawn_C|Getsaw%20armleft _asenemy_pawn)))))
  (bind _output_get_2 (Variables|Default|Setattackrotation (+ 1.8e+02 _output_get)))
  (Utilities|FlowControl|Sequence
    (:then_0
      (Components|MoveComponentTo (Variables|/Game/Blueprints/Boss/Enemy_pawn.Enemy_pawn_C|Getsaw%20armleft _asenemy_pawn) (Variables|/Script/Engine.SceneComponent|GetRelativeLocation (Variables|/Game/Blueprints/Boss/Enemy_pawn.Enemy_pawn_C|Getsaw%20armleft _asenemy_pawn)) (Math|Rotator|MakeRotator _output_get_2 0.0 0.0) false false 2.0 false :!label _label)
      (Development|PrintString "attackleft")
      (AI|BehaviorTree|FinishExecute true))
    (:then_1
      (Utilities|FlowControl|Delay 1.9)
      (goto _label Return))))