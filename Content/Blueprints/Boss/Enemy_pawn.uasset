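; Boss enemy pawn that hurts the slime player and can be moved between stages by teleporting.
; The damage event decrements and prints health, then at zero plays an effect and sound at the body before destroying the actor after a delay.
; Left and right saw colliders call DamagePlayer when they overlap a Slime_Player.
; Left, right, up and down events teleport it by fixed Y or Z offsets, each gated by a DoOnce that resets after a delay.
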(event OnComponentBeginOverlap(sawrightcollider)
  (params (OverlappedComponent :type Primitive%20Component%20Object%20Reference) (OtherActor :type Actor%20Object%20Reference) (OtherComp :type Primitive%20Component%20Object%20Reference) (OtherBodyIndex :type Integer) (bFromSweep :type Boolean) (SweepResult :type Hit%20Result%20Structure%20%28by%20ref%29))
  ;[1 1 1] damage player
  (bind _asslime_player (Utilities|Casting|CastToSlime_Player OtherActor))
  (Default|DamagePlayer _asslime_player))

(event OnComponentBeginOverlap(sawleftcollider)
  (params (OverlappedComponent :type Primitive%20Component%20Object%20Reference) (OtherActor :type Actor%20Object%20Reference) (OtherComp :type Primitive%20Component%20Object%20Reference) (OtherBodyIndex :type Integer) (bFromSweep :type Boolean) (SweepResult :type Hit%20Result%20Structure%20%28by%20ref%29))
  ;[1 1 1] damage player
  (bind _asslime_player (Utilities|Casting|CastToSlime_Player OtherActor))
  (Default|DamagePlayer _asslime_player))

(event Custom|damage
  (bind _body (Variables|Default|Getbody))
  (bind _returnvalue (Transformation|GetWorldLocation _body))
  ;[1 1 1] boss health
  (bind _output_get (Variables|Default|Sethealth (- (Variables|Default|Gethealth) 1.0)))
  (Development|PrintString (Utilities|String|ToString(Float) _output_get))
  (if (<= (Variables|Default|Gethealth) 0.0)
    (Effects|SpawnEmitteratLocation 0 _returnvalue)
    (Audio|PlaySoundatLocation 0 _returnvalue "0, 0, 0" 1.0 1.0 0.0 0 0 0 0)
    (Utilities|FlowControl|Delay 1.0)
    (Actor|DestroyActor)))

(event Custom|left
  (bind _defaultsceneroot (Variables|Default|GetDefaultSceneRoot))
  (bind _returnvalue (Transformation|GetWorldLocation _defaultsceneroot))
  ;[1 1 1] Moves boss to required stage
  (Utilities|FlowControl|DoOnce false :!label _label
    (:Completed
      (Variables|Default|SetReturn%20Value%20X (.x _returnvalue))
      (bind _output_get (Variables|Default|SetReturn%20Value%20Y (.y _returnvalue)))
      (Variables|Default|SetReturn%20Value%20Z (.z _returnvalue))
      (Variables|Default|SetReturn%20Value%20Y (- _output_get 8.1e+02))
      (Transformation|SetActorLocation (Math|Vector|MakeVector (Variables|Default|GetReturn%20Value%20X) (Variables|Default|GetReturn%20Value%20Y) (Variables|Default|GetReturn%20Value%20Z)) false true)
      (Utilities|FlowControl|Delay 1.0)
      (goto _label Reset))))

(event Custom|right
  (bind _defaultsceneroot (Variables|Default|GetDefaultSceneRoot))
  (bind _returnvalue (Transformation|GetWorldLocation _defaultsceneroot))
  ;[1 1 1] Moves boss to required stage
  (Utilities|FlowControl|DoOnce false :!label _label
    (:Completed
      (Variables|Default|SetReturn%20Value%20X (.x _returnvalue))
      (bind _output_get (Variables|Default|SetReturn%20Value%20Y (.y _returnvalue)))
      (Variables|Default|SetReturn%20Value%20Z (.z _returnvalue))
      (Variables|Default|SetReturn%20Value%20Y (+ _output_get 8.1e+02))
      (Transformation|SetActorLocation (Math|Vector|MakeVector (Variables|Default|GetReturn%20Value%20X) (Variables|Default|GetReturn%20Value%20Y) (Variables|Default|GetReturn%20Value%20Z)) false true)
      (Utilities|FlowControl|Delay 1.0)
      (goto _label Reset))))

(event Custom|Up
  (bind _defaultsceneroot (Variables|Default|GetDefaultSceneRoot))
  (bind _returnvalue (Transformation|GetWorldLocation _defaultsceneroot))
  ;[1 1 1] Moves boss to required stage
  (Utilities|FlowControl|DoOnce false :!label _label
    (:Completed
      (Variables|Default|SetReturn%20Value%20X (.x _returnvalue))
      (Variables|Default|SetReturn%20Value%20Y (.y _returnvalue))
      (bind _output_get (Variables|Default|SetReturn%20Value%20Z (.z _returnvalue)))
      (Variables|Default|SetReturn%20Value%20Z (+ 1.3e+03 _output_get))
      (Transformation|SetActorLocation (Math|Vector|MakeVector (Variables|Default|GetReturn%20Value%20X) (Variables|Default|GetReturn%20Value%20Y) (Variables|Default|GetReturn%20Value%20Z)) false true)
      (Utilities|FlowControl|Delay 1.0)
      (goto _label Reset))))

(event Custom|Down
  (bind _defaultsceneroot (Variables|Default|GetDefaultSceneRoot))
  (bind _returnvalue (Transformation|GetWorldLocation _defaultsceneroot))
  ;[1 1 1] Moves boss to required stage
  (Utilities|FlowControl|DoOnce false :!label _label
    (:Completed
      (Variables|Default|SetReturn%20Value%20X (.x _returnvalue))
      (Variables|Default|SetReturn%20Value%20Y (.y _returnvalue))
      (bind _output_get (Variables|Default|SetReturn%20Value%20Z (.z _returnvalue)))
      (Variables|Default|SetReturn%20Value%20Z (- _output_get 1.3e+03))
      (Transformation|SetActorLocation (Math|Vector|MakeVector (Variables|Default|GetReturn%20Value%20X) (Variables|Default|GetReturn%20Value%20Y) (Variables|Default|GetReturn%20Value%20Z)) false true)
      (Utilities|FlowControl|Delay 1.0)
      (goto _label Reset))))

(event EventBeginPlay)

(event Collision|EventActorBeginOverlap
  (params (OtherActor :type Actor%20Object%20Reference)))

(event EventTick
  (params (DeltaSeconds :type Float%20%28single-precision%29)))

(fn ConstructionScript)