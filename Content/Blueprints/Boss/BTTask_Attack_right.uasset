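; Behavior tree task for the boss's right saw-arm attack on Enemy_pawn.
; It reads the SawArmright world roll, snaps the arm's relative roll to that value plus 90 degrees, then restores the stored roll after a short delay and finishes successfully.
; The swing only sets rotation, mixing world-space reads with relative-space writes and zeroing pitch and yaw; its debug print says "attackleft" despite the right arm.
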(event EventReceiveExecuteAI
  (params (OwnerController :type AI%20Controller%20Object%20Reference) (ControlledPawn :type Pawn%20Object%20Reference))
  (bind _asenemy_pawn (Utilities|Casting|CastToEnemy_pawn ControlledPawn))
  (bind _output_get (Variables|Default|Setdefaultrotation (.roll (Transformation|GetWorldRotation (Variables|/Game/Blueprints/Boss/Enemy_pawn.Enemy_pawn_C|GetSawArmright _asenemy_pawn)))))
  (bind _output_get_2 (Variables|Default|Setattackrotation (+ 9e+01 _output_get)))
  (Transformation|SetRelativeRotation (Variables|/Game/Blueprints/Boss/Enemy_pawn.Enemy_pawn_C|GetSawArmright _asenemy_pawn) (Math|Rotator|MakeRotator _output_get_2 0.0 0.0) false false)
  (Utilities|FlowControl|Delay 1.0)
  (Transformation|SetRelativeRotation (Variables|/Game/Blueprints/Boss/Enemy_pawn.Enemy_pawn_C|GetSawArmright _asenemy_pawn) (Math|Rotator|MakeRotator (Variables|Default|Getdefaultrotation) 0.0 0.0) false false)
  (Development|PrintString "attackleft")
  (AI|BehaviorTree|FinishExecute true))